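; PNPickupCoinActor is a coin pickup that spins its mesh and adds one coin to the player pawn that touches it.
; BeginPlay plays a timeline that drives the mesh's yaw and starts a short timer that opens a gate.
; Box overlaps pass through that gate, so pickup waits for the delay, then a PNPlayerPawn gets the coin and the actor destroys itself.
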(event OnComponentBeginOverlap(Box)
  (params (OverlappedComponent :type Primitive%20Component%20Object%20Reference) (OtherActor :type Actor%20Object%20Reference) (OtherComp :type Primitive%20Component%20Object%20Reference) (OtherBodyIndex :type Integer) (bFromSweep :type Boolean) (SweepResult :type Hit%20Result%20Structure%20%28by%20ref%29))
  (Utilities|FlowControl|Gate true
    (:Exit
      (bind _aspnplayer_pawn (Utilities|Casting|CastToPNPlayerPawn OtherActor))
      (Default|AddCoin _aspnplayer_pawn 1)
      (Actor|DestroyActor))))

(event Custom|EnablePickUp
  (Utilities|FlowControl|Gate true) ; enters at Open
)

(event EventBeginPlay
  (Utilities|Time|SetTimerbyFunctionName 0 "EnablePickUp" 0.5)
  (bind _coinyaw (Timeline|CoinRotationTimeline Play)
    (:Update
      (Transformation|SetRelativeRotation (Variables|Debug|GetStaticMeshComponent) (Math|Rotator|MakeRotator 0.0 0.0 _coinyaw) false false))))

(event Collision|EventActorBeginOverlap
  (params (OtherActor :type Actor%20Object%20Reference)))

(event EventTick
  (params (DeltaSeconds :type Float%20%28single-precision%29)))

(fn ConstructionScript)